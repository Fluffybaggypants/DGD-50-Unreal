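; Dialogue component for the Mouse character, holding a short branching conversation that greets the player and offers to talk.
; It overrides Dialogue, calls the parent, then switches on the tree index and chains AddDialogue calls, advancing on Pass Through and branching by chosen option.
; Declining leads to a farewell that clears progress and closes the conversation.
; Accepting opens a cave question whose options lead nowhere yet; debug prints remain.
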(fn `Dialogue`
  (`parent.Dialogue`)
  (switch `int` (`self.DialogueTree Index`)
    (:`0`
      (bind (_state _optionindex) (`self.AddDialogue` "Mouse" "Ah. Nice to meet you! Shall we talk?" (`|MakeArray` "Yes." "No" :!type "Text")))
      (`KismetSystemLibrary.PrintString` (`KismetStringLibrary.Conv_IntToString` _optionindex))
      (switch `/Game/Blueprints/Dialogue/Enum_DialogueState` _state
        (:`NewEnumerator0`
          (`KismetSystemLibrary.PrintString` "Car")
          (switch `int` _optionindex
            (:`0`
              (bind (_state_2 _optionindex_2) (`self.AddDialogue` "Mouse" "What do you want to know about this cave?" (`|MakeArray` "Yes.Tell me about the cave." "Goodbye" :!type "Text")))
              (switch `/Game/Blueprints/Dialogue/Enum_DialogueState` _state_2
                (:`NewEnumerator0`
                  (switch `int` _optionindex_2))))
            (:`1`
              (bind _state_3 (`self.AddDialogue` "Mouse" "Nice knowing you!" (`|MakeArray` "Continue" :!type "Text")))
              (switch `/Game/Blueprints/Dialogue/Enum_DialogueState` _state_3
                (:`NewEnumerator0`
                  (`self.ClearDialogueProgress`)
                  (`self.CloseConversation`))))))))))